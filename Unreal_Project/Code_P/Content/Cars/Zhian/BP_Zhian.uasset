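; BP_Zhian is a drivable car Blueprint that handles player driving and camera look.
; Each Tick runs two functions, polling input axes rather than binding to input events.
; Vehicle_Input feeds throttle, brake, steering and handbrake to the vehicle movement component, turning the handbrake axis into a boolean.
; Camera_Input applies look axes as relative pitch and yaw increments to the spring arm, without delta-time scaling.
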(event EventTick
  (params (DeltaSeconds :type Float%20%28single-precision%29))
  (CallFunction|VehicleInput)
  (CallFunction|CameraInput))

(fn ConstructionScript)

(fn VehicleInput
  (bind _vehiclemovementcomponent (Variables|Default|GetVehicleMovementComponent))
  (Class|ChaosVehicleMovementComponent|SetThrottleInput _vehiclemovementcomponent (Input|AxisValues|GetThrottle_Input))
  (Class|ChaosVehicleMovementComponent|SetBrakeInput _vehiclemovementcomponent (Input|AxisValues|GetBrake_Input))
  (Class|ChaosVehicleMovementComponent|SetSteeringInput _vehiclemovementcomponent (Input|AxisValues|GetSteering_Input))
  (Class|ChaosVehicleMovementComponent|SetHandbrakeInput _vehiclemovementcomponent (== (Input|AxisValues|GetHandbrake_Input) 1.0)))

(fn CameraInput
  (Transformation|AddRelativeRotation (Variables|Default|GetSpringArm) (Math|Rotator|MakeRotator 0.0 (Input|AxisValues|GetLookUp) (Input|AxisValues|GetLookRight)) false false))